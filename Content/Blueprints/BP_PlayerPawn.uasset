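; Player pawn with touch-drag look, local HUD setup and debug health readouts.
; Touch movement deltas, scaled by TurnSpeed and frame time, feed controller pitch and yaw input.
; For the locally controlled pawn, BeginPlay adds the crosshair and BP_FPP_UI widgets, and Tick prints current health on screen.
; The OnHealthChanged event draws each health delta as debug text at the pawn's location.
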(event OnHealthChanged(SHealth)
  (params (OwningHealthComp :type S%20Health%20Component%20Object%20Reference) (Health :type Float%20%28single-precision%29) (HealthDelta :type Float%20%28single-precision%29) (DamageType :type Damage%20Type%20Object%20Reference) (InstigatedBy :type Controller%20Object%20Reference) (DamageCauser :type Actor%20Object%20Reference))
  (Rendering|Debug|DrawDebugString (Transformation|GetActorLocation) (Utilities|String|ToString(Float) HealthDelta) 0 "(R=1.000000,G=1.000000,B=1.000000,A=1.000000)"))

(event EventBeginPlay
  (if (Pawn|IsLocallyControlled)
    (Utilities|FlowControl|Sequence
      (:then_0
        (bind _returnvalue (UserInterface|CreateWidget "/Game/Blueprints/Widget/WBP_Crosshair.WBP_Crosshair_C"))
        (UserInterface|Viewport|AddtoViewport _returnvalue 0))
      (:then_1
        (bind _returnvalue_2 (UserInterface|CreateWidget "/Game/Blueprints/Widget/BP_FPP_UI.BP_FPP_UI_C"))
        (UserInterface|Viewport|AddtoViewport _returnvalue_2 0)))))

(event Collision|EventActorBeginOverlap
  (params (OtherActor :type Actor%20Object%20Reference)))

(event EventTick
  (params (DeltaSeconds :type Float%20%28single-precision%29))
  (if (Pawn|IsLocallyControlled)
    (Development|PrintString (Utilities|String|ToString(Float) (Variables|/Script/FPSGame.SHealthComponent|GetHealth (Variables|Default|GetHealthComp))) true true "(R=1.000000,G=0.871950,B=0.000000,A=1.000000)" 0.0)))

(event Input|TouchEvents|InputTouch
  (params (Location :type Vector) (FingerIndex :type ETouchIndex%20Enum))
  (bind _returnvalue (Utilities|Time|GetWorldDeltaSeconds))
  ;[1 1 1] 左右移动视角
  (:Pressed
    (Variables|Default|SetTouch%20Start Location))
  (:Moved
    (Pawn|Input|AddControllerPitchInput (* (.Y (Math|Vector|BreakVector (- (Variables|Default|GetTouch%20Start) Location))) (Variables|Default|GetTurnSpeed) _returnvalue))
    (Pawn|Input|AddControllerYawInput (* (.X (Math|Vector|BreakVector (- (Variables|Default|GetTouch%20Start) Location))) (Variables|Default|GetTurnSpeed) _returnvalue))
    (Variables|Default|SetTouch%20Start Location)))

(fn ConstructionScript)